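; BP_Magnet is a lesson magnet actor that moves actors overlapping its Box component.
; Each tick it offsets every overlapping actor except itself, with sweep, at Strength scaled by delta time.
; The direction is the normalized vector from its TargetPoint component to the magnet's own location, so all affected actors move in parallel rather than converging on a point.
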(event `self.ReceiveTick`
  (params (DeltaSeconds :type "Float (single-precision)"))
  (for _array_element (`PrimitiveComponent.GetOverlappingActors` (`self.Box`) null)
    (if (!= _array_element self)
      (`self.K2_AddActorWorldOffset` _array_element (* (`KismetMathLibrary.Normal` (- (`self.K2_GetActorLocation`) (`SceneComponent.K2_GetComponentLocation` (`self.TargetPoint`)))) (`self.Strength`) DeltaSeconds) true false))))

(fn `UserConstructionScript`)