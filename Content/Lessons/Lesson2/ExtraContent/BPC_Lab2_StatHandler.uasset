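; BPC_Lab2_StatHandler is a lesson component that tracks health and stamina values.
; SetHealth and SetStamina clamp each value between zero and its maximum, then fire OnHealthChange or OnStaminaChange dispatchers with the new value.
; The TakeDamage event subtracts damage from health through SetHealth, so damage follows the same clamp and notification path.
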(event `Take Damage`
  (params (Damage :type "Float (double-precision)"))
  (`self.Set Health` (- (`self.Health`) Damage)))

(fn `Set Health`
  (params (Value :type "Float (double-precision)"))
  (bind _output_get (set `self.Health` (`KismetMathLibrary.FClamp` Value 0.0 (`self.MaxHealth`))))
  (`self.OnHealthChange` _output_get))

(fn `Set Stamina`
  (params (Value :type "Float (double-precision)"))
  (bind _output_get (set `self.Stamina` (`KismetMathLibrary.FClamp` Value 0.0 (`self.MaxStamina`))))
  (`self.OnStaminaChange` _output_get))