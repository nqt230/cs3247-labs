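; BP_Lab2_Character2 is a Lesson 2 lab player character that delegates movement, skills and health to handler components.
; BeginPlay adds an Enhanced Input mapping context, then input events forward move, look and jump to the movement handler and primary/secondary actions to the skill handler.
; Sprint press and release share one FlipFlop, whose toggled state sets the movement handler's sprint flag.
; Incoming damage passes to the stat handler.
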(event `self.ReceiveBeginPlay`
  ; Initialization
  (bind _asplayer_controller (cast `PlayerController` (`self.GetController`)))
  (`EnhancedInputSubsystemInterface.AddMappingContext` (pcsubsystem `EnhancedInputLocalPlayerSubsystem` _asplayer_controller) "/Game/Lessons/Lesson2/ExtraContent/InputActions/InputMappingContext.InputMappingContext" 0 (struct)))

(event `EnhancedInput|/Game/Lessons/Lesson2/ExtraContent/InputActions/IA_Move_UD`
  (params (ActionValue :type "Float (double-precision)") (ElapsedSeconds :type "Float (double-precision)") (TriggeredSeconds :type "Float (double-precision)") (InputAction :type "InputAction Object Reference" :default "/Game/Lessons/Lesson2/ExtraContent/InputActions/IA_Move_UD.IA_Move_UD"))
  ; Movement
  (:`Triggered`
    (`/Game/Lessons/Lesson2/ExtraContent/BPC_Lab2_MovementHandler.HandleMoveUD` (`self.BPC_Lab2_MovementHandler`) ActionValue)))

(event `EnhancedInput|/Game/Lessons/Lesson2/ExtraContent/InputActions/IA_Look_Yaw`
  (params (ActionValue :type "Float (double-precision)") (ElapsedSeconds :type "Float (double-precision)") (TriggeredSeconds :type "Float (double-precision)") (InputAction :type "InputAction Object Reference" :default "/Game/Lessons/Lesson2/ExtraContent/InputActions/IA_Look_Yaw.IA_Look_Yaw"))
  ; Movement
  (:`Triggered`
    (`/Game/Lessons/Lesson2/ExtraContent/BPC_Lab2_MovementHandler.HandleLookYaw` (`self.BPC_Lab2_MovementHandler`) ActionValue)))

(event `EnhancedInput|/Game/Lessons/Lesson2/ExtraContent/InputActions/IA_Look_Pitch`
  (params (ActionValue :type "Float (double-precision)") (ElapsedSeconds :type "Float (double-precision)") (TriggeredSeconds :type "Float (double-precision)") (InputAction :type "InputAction Object Reference" :default "/Game/Lessons/Lesson2/ExtraContent/InputActions/IA_Look_Pitch.IA_Look_Pitch"))
  ; Movement
  (:`Triggered`
    (`/Game/Lessons/Lesson2/ExtraContent/BPC_Lab2_MovementHandler.HandleLookPitch` (`self.BPC_Lab2_MovementHandler`) ActionValue)))

(event `EnhancedInput|/Game/Lessons/Lesson2/ExtraContent/InputActions/IA_Move_LR`
  (params (ActionValue :type "Float (double-precision)") (ElapsedSeconds :type "Float (double-precision)") (TriggeredSeconds :type "Float (double-precision)") (InputAction :type "InputAction Object Reference" :default "/Game/Lessons/Lesson2/ExtraContent/InputActions/IA_Move_LR.IA_Move_LR"))
  ; Movement
  (:`Triggered`
    (`/Game/Lessons/Lesson2/ExtraContent/BPC_Lab2_MovementHandler.HandleMoveLR` (`self.BPC_Lab2_MovementHandler`) ActionValue)))

(event `EnhancedInput|/Game/Lessons/Lesson2/ExtraContent/InputActions/IA_Jump`
  (params (ActionValue :type Boolean) (ElapsedSeconds :type "Float (double-precision)") (TriggeredSeconds :type "Float (double-precision)") (InputAction :type "InputAction Object Reference" :default "/Game/Lessons/Lesson2/ExtraContent/InputActions/IA_Jump.IA_Jump"))
  (bind _bpc_lab2_movementhandler (`self.BPC_Lab2_MovementHandler`))
  ; Movement
  (:`Started`
    (`/Game/Lessons/Lesson2/ExtraContent/BPC_Lab2_MovementHandler.Jump` _bpc_lab2_movementhandler))
  (:`Completed`
    (`/Game/Lessons/Lesson2/ExtraContent/BPC_Lab2_MovementHandler.StopJump` _bpc_lab2_movementhandler)))

(event `EnhancedInput|/Game/Lessons/Lesson2/ExtraContent/InputActions/IA_Sprint`
  (params (ActionValue :type Boolean) (ElapsedSeconds :type "Float (double-precision)") (TriggeredSeconds :type "Float (double-precision)") (InputAction :type "InputAction Object Reference" :default "/Game/Lessons/Lesson2/ExtraContent/InputActions/IA_Sprint.IA_Sprint"))
  ; Movement
  (:`Started`
    (bind _isa (`/Engine/EditorBlueprintResources/StandardMacros.FlipFlop` :!label _label)
      (:`A`
        _)
      (:`B`
        _))
    (`/Game/Lessons/Lesson2/ExtraContent/BPC_Lab2_MovementHandler.Set Is Sprinting` (`self.BPC_Lab2_MovementHandler`) _isa))
  (:`Completed`
    (goto _label)))

(event `EnhancedInput|/Game/Lessons/Lesson2/ExtraContent/InputActions/IA_Action_Primary`
  (params (ActionValue :type Boolean) (ElapsedSeconds :type "Float (double-precision)") (TriggeredSeconds :type "Float (double-precision)") (InputAction :type "InputAction Object Reference" :default "/Game/Lessons/Lesson2/ExtraContent/InputActions/IA_Action_Primary.IA_Action_Primary"))
  ; Skill
  (:`Triggered`
    (`/Game/Lessons/Lesson2/ExtraContent/BPC_Lab2_SkillHandler.Primary Skill` (`self.BPC_Lab2_SkillHandler`))))

(event `EnhancedInput|/Game/Lessons/Lesson2/ExtraContent/InputActions/IA_Action_Secondary`
  (params (ActionValue :type Boolean) (ElapsedSeconds :type "Float (double-precision)") (TriggeredSeconds :type "Float (double-precision)") (InputAction :type "InputAction Object Reference" :default "/Game/Lessons/Lesson2/ExtraContent/InputActions/IA_Action_Secondary.IA_Action_Secondary"))
  ; Skill
  (:`Triggered`
    (`/Game/Lessons/Lesson2/ExtraContent/BPC_Lab2_SkillHandler.Secondary Skill` (`self.BPC_Lab2_SkillHandler`))))

(event `Take Damage`
  (params (Damage :type "Float (double-precision)"))
  ; Health
  (`/Game/Lessons/Lesson2/ExtraContent/BPC_Lab2_StatHandler.Take Damage` (`self.BPC_Lab2_StatHandler`) Damage))

(fn `UserConstructionScript`)