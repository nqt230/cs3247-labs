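; Actor component for a Lesson 2 lab that handles a primary and a secondary skill, playing effects and sounds at its owner's location.
; The primary skill spawns a neon explosion and uses a random looping MultiGate to pick one of three laser sounds.
; The secondary skill spawns an asteroid explosion with sound, using an initially open Gate that closes on use and reopens after a cooldown delay.
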(event `Primary Skill`
  (bind _returnvalue (`Actor.K2_GetActorLocation` (`self.GetOwner`)))
  (`GameplayStatics.SpawnEmitterAtLocation` "/Game/Effects/Particles/Explosion/P_NeonExplosion.P_NeonExplosion" _returnvalue)
  (`|MultiGate` true true
    (:`Out 0`
      (`GameplayStatics.PlaySoundAtLocation` "/Game/Audio/SoundWaves/Effect/SW_Laser_1.SW_Laser_1" _returnvalue (struct) 1.0 1.0 0.0 null null null null))
    (:`Out 1`
      (`GameplayStatics.PlaySoundAtLocation` "/Game/Audio/SoundWaves/Effect/SW_Laser_2.SW_Laser_2" _returnvalue (struct) 1.0 1.0 0.0 null null null null))
    (:`Out 2`
      (`GameplayStatics.PlaySoundAtLocation` "/Game/Audio/SoundWaves/Effect/SW_Laser_3.SW_Laser_3" _returnvalue (struct) 1.0 1.0 0.0 null null null null))))

(event `Secondary Skill`
  (bind _returnvalue (`Actor.K2_GetActorLocation` (`self.GetOwner`)))
  (`/Engine/EditorBlueprintResources/StandardMacros.Gate` false :!label _label
    (:`Exit`
      (`|ExecutionSequence`
        (:`then_0`
          (`GameplayStatics.SpawnEmitterAtLocation` "/Game/Effects/Particles/Explosion/P_AsteroidExplosion.P_AsteroidExplosion" _returnvalue)
          (`GameplayStatics.PlaySoundAtLocation` "/Game/Audio/SoundWaves/Effect/SW_Explosion_1.SW_Explosion_1" _returnvalue (struct) 1.0 1.0 0.0 null null null null))
        (:`then_1`
          (goto _label :!via `Close`))
        (:`then_2`
          (`KismetSystemLibrary.Delay` (`self.SecondaryCooldown`))
          (goto _label :!via `Open`))))))