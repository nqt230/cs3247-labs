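; Lesson 2 example Blueprint that demonstrates flow control nodes, each in its own event that prints strings to show the execution path.
; It covers Sequence, Select on a visibility enum, FlipFlop as a pause toggle, looping MultiGate as an attack cycle, and DoOnce for lazy initialization.
; The two Gate events share one gate: one passes an action through it, the other closes it for a one-second cooldown.
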(event `Sequence Example`
  (`|ExecutionSequence`
    (:`then_0`
      (`KismetSystemLibrary.PrintString` "A")
      (`KismetSystemLibrary.PrintString` "B")
      (`KismetSystemLibrary.PrintString` "C")
      (`KismetSystemLibrary.PrintString` "D"))
    (:`then_1`
      (`KismetSystemLibrary.PrintString` "E")
      (`KismetSystemLibrary.PrintString` "F")
      (`KismetSystemLibrary.PrintString` "G")
      (`KismetSystemLibrary.PrintString` "H"))))

(event `Select Example`
  (params (NewParam :type "ESlateVisibility Enum" :default "Visible"))
  (`KismetSystemLibrary.PrintString` (select `ESlateVisibility` NewParam :`Visible` "Visible" :`Collapsed` "Collapsed" :`Hidden` "Hidden" :`HitTestInvisible` "Visible no raycast recursive" :`SelfHitTestInvisible` "Visible no raycast self")))

(event `FlipFlop Example`
  (`/Engine/EditorBlueprintResources/StandardMacros.FlipFlop`
    (:`A`
      (`KismetSystemLibrary.PrintString` "Pause Game"))
    (:`B`
      (`KismetSystemLibrary.PrintString` "Unpause Game"))))

(event `Gate Example 1`
  (`/Engine/EditorBlueprintResources/StandardMacros.Gate` false :!label _label
    (:`Exit`
      (`KismetSystemLibrary.PrintString` "DoAction")
      (`self.ExampleEvent5`))))

(event `Gate Example 2`
  (`KismetSystemLibrary.PrintString` "StartCooldown")
  (`|ExecutionSequence`
    (:`then_0`
      (goto _label :!via `Close`))
    (:`then_1`
      (`KismetSystemLibrary.Delay` 1.0)
      (`KismetSystemLibrary.PrintString` "EndCooldown")
      (goto _label :!via `Open`))))

(event `MultiGate Example`
  (`KismetSystemLibrary.PrintString` "Attack input")
  (`|MultiGate` false true
    (:`Out 0`
      (`KismetSystemLibrary.PrintString` "Perform Attack 1"))
    (:`Out 1`
      (`KismetSystemLibrary.PrintString` "Perform Attack 2"))
    (:`Out 2`
      (`KismetSystemLibrary.PrintString` "Perform Attack 3"))))

(event `DoOnce Example`
  (`|ExecutionSequence`
    (:`then_0`
      (`/Engine/EditorBlueprintResources/StandardMacros.DoOnce` false
        (:`Completed`
          (`KismetSystemLibrary.PrintString` "Lazy loading/initialization"))))
    (:`then_1`
      (`KismetSystemLibrary.PrintString` "Some logic"))))

(fn `ExampleEvent5`)

(fn `UserConstructionScript`)