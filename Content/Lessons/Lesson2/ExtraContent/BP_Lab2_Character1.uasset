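; Lesson 2 lab player character with Enhanced Input movement, look, jump, sprint and two effect-only skills.
; Movement follows camera axes and toggles orient-to-movement, while a FlipFlop on sprint press and release switches walk speed.
; Primary skill spawns an explosion with a random laser sound; secondary uses a Gate and Delay as cooldown.
; Clamped Health and Stamina setters broadcast percentages, with damage feeding Health; nothing here changes Stamina.
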(event `self.ReceiveBeginPlay`
  ; Initialization
  (bind _asplayer_controller (cast `PlayerController` (`self.GetController`)))
  (`EnhancedInputSubsystemInterface.AddMappingContext` (pcsubsystem `EnhancedInputLocalPlayerSubsystem` _asplayer_controller) "/Game/InputActions/InputMappingContext.InputMappingContext" 0 (struct)))

(event `Take Damage`
  (params (Damage :type "Float (double-precision)"))
  ; Health
  (`self.Set Health` (- (`self.Health`) Damage)))

(event `Set Health Event`
  (params (Value :type "Float (double-precision)"))
  ; Health
  (set `self.Health` (`KismetMathLibrary.FClamp` Value 0.0 (`self.MaxHealth`)))
  (`self.OnHealthChange` (`self.Get Health Percentage`)))

(event `EnhancedInput|/Game/InputActions/IA_Move_UD`
  (params (ActionValue :type "Float (double-precision)") (ElapsedSeconds :type "Float (double-precision)") (TriggeredSeconds :type "Float (double-precision)") (InputAction :type "InputAction Object Reference" :default "/Game/InputActions/IA_Move_UD.IA_Move_UD"))
  ; Movement
  (:`Triggered`
    (`self.AddMovementInput` (`self.GetActorForwardVector` (`GameplayStatics.GetPlayerCameraManager` 0)) ActionValue)
    (set `CharacterMovementComponent.bOrientRotationToMovement` (not (or (!= ActionValue 0.0) (!= (stale `EnhancedInput|/Game/InputActions/IA_Move_LR` ActionValue) 0.0))) (`self.CharacterMovement`) :!label _label)))

(event `EnhancedInput|/Game/InputActions/IA_Look_Yaw`
  (params (ActionValue :type "Float (double-precision)") (ElapsedSeconds :type "Float (double-precision)") (TriggeredSeconds :type "Float (double-precision)") (InputAction :type "InputAction Object Reference" :default "/Game/InputActions/IA_Look_Yaw.IA_Look_Yaw"))
  ; Movement
  (:`Triggered`
    (`self.AddControllerYawInput` ActionValue)))

(event `EnhancedInput|/Game/InputActions/IA_Look_Pitch`
  (params (ActionValue :type "Float (double-precision)") (ElapsedSeconds :type "Float (double-precision)") (TriggeredSeconds :type "Float (double-precision)") (InputAction :type "InputAction Object Reference" :default "/Game/InputActions/IA_Look_Pitch.IA_Look_Pitch"))
  ; Movement
  (:`Triggered`
    (`self.AddControllerPitchInput` ActionValue)))

(event `EnhancedInput|/Game/InputActions/IA_Move_LR`
  (params (ActionValue :type "Float (double-precision)") (ElapsedSeconds :type "Float (double-precision)") (TriggeredSeconds :type "Float (double-precision)") (InputAction :type "InputAction Object Reference" :default "/Game/InputActions/IA_Move_LR.IA_Move_LR"))
  ; Movement
  (:`Triggered`
    (`self.AddMovementInput` (`self.GetActorRightVector` (`GameplayStatics.GetPlayerCameraManager` 0)) ActionValue)
    (goto _label)))

(event `EnhancedInput|/Game/InputActions/IA_Jump`
  (params (ActionValue :type Boolean) (ElapsedSeconds :type "Float (double-precision)") (TriggeredSeconds :type "Float (double-precision)") (InputAction :type "InputAction Object Reference" :default "/Game/InputActions/IA_Jump.IA_Jump"))
  ; Movement
  (:`Started`
    (`self.Jump`))
  (:`Completed`
    (`self.StopJumping`)))

(event `EnhancedInput|/Game/InputActions/IA_Sprint`
  (params (ActionValue :type Boolean) (ElapsedSeconds :type "Float (double-precision)") (TriggeredSeconds :type "Float (double-precision)") (InputAction :type "InputAction Object Reference" :default "/Game/InputActions/IA_Sprint.IA_Sprint"))
  ; Movement
  (:`Started`
    (bind _isa (`/Engine/EditorBlueprintResources/StandardMacros.FlipFlop` :!label _label_2)
      (:`A`
        _)
      (:`B`
        _))
    (`self.Set Is Sprinting` _isa))
  (:`Completed`
    (goto _label_2)))

(event `EnhancedInput|/Game/InputActions/IA_Action_Primary`
  (params (ActionValue :type Boolean) (ElapsedSeconds :type "Float (double-precision)") (TriggeredSeconds :type "Float (double-precision)") (InputAction :type "InputAction Object Reference" :default "/Game/InputActions/IA_Action_Primary.IA_Action_Primary"))
  (bind _returnvalue (`self.K2_GetActorLocation`))
  ; Skill
  (:`Triggered`
    (`GameplayStatics.SpawnEmitterAtLocation` "/Game/Effects/Particles/Explosion/P_NeonExplosion.P_NeonExplosion" _returnvalue)
    (`|MultiGate` true true
      (:`Out 0`
        (`GameplayStatics.PlaySoundAtLocation` "/Game/Audio/SoundWaves/Effect/SW_Laser_1.SW_Laser_1" _returnvalue (struct) 1.0 1.0 0.0 null null null null))
      (:`Out 1`
        (`GameplayStatics.PlaySoundAtLocation` "/Game/Audio/SoundWaves/Effect/SW_Laser_2.SW_Laser_2" _returnvalue (struct) 1.0 1.0 0.0 null null null null))
      (:`Out 2`
        (`GameplayStatics.PlaySoundAtLocation` "/Game/Audio/SoundWaves/Effect/SW_Laser_3.SW_Laser_3" _returnvalue (struct) 1.0 1.0 0.0 null null null null)))))

(event `EnhancedInput|/Game/InputActions/IA_Action_Secondary`
  (params (ActionValue :type Boolean) (ElapsedSeconds :type "Float (double-precision)") (TriggeredSeconds :type "Float (double-precision)") (InputAction :type "InputAction Object Reference" :default "/Game/InputActions/IA_Action_Secondary.IA_Action_Secondary"))
  (bind _returnvalue (`self.K2_GetActorLocation`))
  ; Skill
  (:`Triggered`
    (`/Engine/EditorBlueprintResources/StandardMacros.Gate` false :!label _label_3
      (:`Exit`
        (`|ExecutionSequence`
          (:`then_0`
            (`GameplayStatics.SpawnEmitterAtLocation` "/Game/Effects/Particles/Explosion/P_AsteroidExplosion.P_AsteroidExplosion" _returnvalue)
            (`GameplayStatics.PlaySoundAtLocation` "/Game/Audio/SoundWaves/Effect/SW_Explosion_1.SW_Explosion_1" _returnvalue (struct) 1.0 1.0 0.0 null null null null))
          (:`then_1`
            (goto _label_3 :!via `Close`))
          (:`then_2`
            (`KismetSystemLibrary.Delay` (`self.SecondaryCooldown`))
            (goto _label_3 :!via `Open`)))))))

(fn `Get Health Percentage`
  (returns (Value :type "Float (double-precision)"))
  (return (`KismetMathLibrary.SafeDivide` (`self.Health`) (`self.MaxHealth`))))

(fn `Get Stamina Percentage`
  (returns (Value :type "Float (double-precision)"))
  (return (`KismetMathLibrary.SafeDivide` (`self.Stamina`) (`self.MaxStamina`))))

(fn `Set Health`
  (params (Value :type "Float (double-precision)"))
  (returns (NewValue :type "Float (double-precision)"))
  (bind _output_get (set `self.Health` (`KismetMathLibrary.FClamp` Value 0.0 (`self.MaxHealth`))))
  (`self.OnHealthChange` (`self.Get Health Percentage`))
  (return _output_get))

(fn `Set Is Sprinting`
  (params (`Is Sprinting` :type Boolean))
  (bind _output_get (set `self.IsSprinting` `Is Sprinting`))
  (set `CharacterMovementComponent.MaxWalkSpeed` (`KismetMathLibrary.SelectFloat` (`self.SprintSpeed`) (`self.WalkSpeed`) _output_get) (`self.CharacterMovement`)))

(fn `Set Stamina`
  (params (Value :type "Float (double-precision)"))
  (set `self.Stamina` (`KismetMathLibrary.FClamp` Value 0.0 (`self.MaxStamina`)))
  (`self.OnStaminaChange` (`self.Get Stamina Percentage`)))

(fn `UserConstructionScript`)