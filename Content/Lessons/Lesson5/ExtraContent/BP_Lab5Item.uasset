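; Lesson 5 item actor that takes its data and mesh from the DT_Items data table.
; The construction script looks up the ItemId row, stores it in ItemData, synchronously loads the soft-referenced ItemModel and applies it to StaticMesh.
; An asynchronous version of the same lookup and load sits unconnected in the event graph, where BeginPlay does nothing.
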(event `self.ReceiveBeginPlay`)

(fn `UserConstructionScript`
  (bind _returnvalue (`|GetDataTableRow` "/Game/Data/DT_Items.DT_Items" (`self.ItemId`))
    (:`then`
      (set `self.ItemData` _returnvalue)
      (bind (_itemname _itemdesc _itemicon _itemmodel) (break `ItemData` _returnvalue))
      (`KismetSystemLibrary.LoadAsset_Blocking` _itemmodel)
      (`StaticMeshComponent.SetStaticMesh` (`self.StaticMesh`) (`|ConvertAsset` _itemmodel)))))