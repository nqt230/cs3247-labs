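; Player character for Lesson 5 that takes its health, stamina, speed, jump and async-loaded mesh from a CharacterData asset.
; Enhanced Input drives movement, look, jump and sprint, which triples walk speed and drains stamina until it runs out.
; Each tick a camera line trace picks a BP_Lab5Item as interaction target, which the E key activates.
; Setters clamp values and fire change events for health, stamina and target.
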(event `self.ReceiveBeginPlay`
  (bind _characterdata (`self.CharacterData`))
  ; Initialization
  (bind _asplayer_controller (cast `PlayerController` (`self.GetController`)))
  (`EnhancedInputSubsystemInterface.AddMappingContext` (pcsubsystem `EnhancedInputLocalPlayerSubsystem` _asplayer_controller) "/Game/InputActions/InputMappingContext.InputMappingContext" 0 (struct))
  (set `self.CurrentHealth` (`/Game/Lessons/Lesson4/ExtraContent/BP_Lab4CharacterData.MaxHealth` _characterdata))
  (set `self.CurrentStamina` (`/Game/Lessons/Lesson4/ExtraContent/BP_Lab4CharacterData.MaxStamina` _characterdata))
  (`self.Initialize`))

(event `Initialize`
  (bind _model (`/Game/Lessons/Lesson4/ExtraContent/BP_Lab4CharacterData.Model` (`self.CharacterData`)))
  ; Initialization
  (`|ExecutionSequence`
    (:`then_0`
      (set `CharacterMovementComponent.JumpZVelocity` (`/Game/Lessons/Lesson4/ExtraContent/BP_Lab4CharacterData.JumpSpeed` (`self.CharacterData`)) (`self.CharacterMovement`))
      (`self.Set Is Sprinting` (`self.IsSprinting`))
      (`self.Set Health` (`self.CurrentHealth`))
      (`self.Set Stamina` (`self.CurrentStamina`)))
    (:`then_1`
      (`|LoadAsset` _model
        (:`Completed`
          (`SkeletalMeshComponent.SetSkeletalMeshAsset` (`self.Mesh`) (`|ConvertAsset` _model)))))))

(event `self.ReceiveTick`
  (params (DeltaSeconds :type "Float (single-precision)"))
  (bind _camera (`self.Camera`))
  (bind _returnvalue (`SceneComponent.K2_GetComponentLocation` _camera))
  (`|ExecutionSequence`
    (:`then_0`
      ; Stamina
      (`self.Set Stamina` (+ (`self.CurrentStamina`) (* (`KismetMathLibrary.SelectFloat` -10.0 5.0 (`self.IsSprinting`)) DeltaSeconds)))
      (if (and (<= (`self.CurrentStamina`) 0.0) (`self.IsSprinting`))
        (`self.Set Is Sprinting` false)))
    (:`then_1`
      ; Interact
      (bind _outhit (`KismetSystemLibrary.LineTraceSingleForObjects` _returnvalue (+ _returnvalue (* (`SceneComponent.GetForwardVector` _camera) 500.0)) (`|MakeArray` "ObjectTypeQuery1" "ObjectTypeQuery2" :!type "EObjectTypeQuery Enum")))
      (bind (_bblockinghit _binitialoverlap _time _distance _location _impactpoint _normal _impactnormal _physmat _hitactor) (`GameplayStatics.BreakHitResult` _outhit))
      (`/Engine/EditorBlueprintResources/StandardMacros.IsValid` _hitactor
        (:`Is Valid`
          (bind _asbp_lab_5item (cast `/Game/Lessons/Lesson5/ExtraContent/BP_Lab5Item` _hitactor))
          (`self.Set Interaction Target` _asbp_lab_5item))
        (:`Is Not Valid`
          (`self.Set Interaction Target` null))))))

(event `EnhancedInput|/Game/InputActions/IA_Move_UD`
  (params (ActionValue :type "Float (double-precision)") (ElapsedSeconds :type "Float (double-precision)") (TriggeredSeconds :type "Float (double-precision)") (InputAction :type "InputAction Object Reference" :default "/Game/InputActions/IA_Move_UD.IA_Move_UD"))
  ; Movement
  (:`Triggered`
    (`self.AddMovementInput` (`self.GetActorForwardVector` (`GameplayStatics.GetPlayerCameraManager` 0)) ActionValue)
    (set `CharacterMovementComponent.bOrientRotationToMovement` (not (or (!= ActionValue 0.0) (!= (stale `EnhancedInput|/Game/InputActions/IA_Move_LR` ActionValue) 0.0))) (`self.CharacterMovement`) :!label _label))
  (:`Completed`
    (goto _label)))

(event `EnhancedInput|/Game/InputActions/IA_Look_Yaw`
  (params (ActionValue :type "Float (double-precision)") (ElapsedSeconds :type "Float (double-precision)") (TriggeredSeconds :type "Float (double-precision)") (InputAction :type "InputAction Object Reference" :default "/Game/InputActions/IA_Look_Yaw.IA_Look_Yaw"))
  ; Movement
  (:`Triggered`
    (`self.AddControllerYawInput` (* ActionValue (`GameplayStatics.GetWorldDeltaSeconds`) 45.0))))

(event `EnhancedInput|/Game/InputActions/IA_Look_Pitch`
  (params (ActionValue :type "Float (double-precision)") (ElapsedSeconds :type "Float (double-precision)") (TriggeredSeconds :type "Float (double-precision)") (InputAction :type "InputAction Object Reference" :default "/Game/InputActions/IA_Look_Pitch.IA_Look_Pitch"))
  ; Movement
  (:`Triggered`
    (`self.AddControllerPitchInput` (* (`GameplayStatics.GetWorldDeltaSeconds`) ActionValue 45.0))))

(event `EnhancedInput|/Game/InputActions/IA_Move_LR`
  (params (ActionValue :type "Float (double-precision)") (ElapsedSeconds :type "Float (double-precision)") (TriggeredSeconds :type "Float (double-precision)") (InputAction :type "InputAction Object Reference" :default "/Game/InputActions/IA_Move_LR.IA_Move_LR"))
  ; Movement
  (:`Triggered`
    (`self.AddMovementInput` (`self.GetActorRightVector` (`GameplayStatics.GetPlayerCameraManager` 0)) ActionValue)
    (goto _label))
  (:`Completed`
    (goto _label)))

(event `EnhancedInput|/Game/InputActions/IA_Jump`
  (params (ActionValue :type Boolean) (ElapsedSeconds :type "Float (double-precision)") (TriggeredSeconds :type "Float (double-precision)") (InputAction :type "InputAction Object Reference" :default "/Game/InputActions/IA_Jump.IA_Jump"))
  ; Movement
  (:`Started`
    (`self.Jump`))
  (:`Completed`
    (`self.StopJumping`)))

(event `EnhancedInput|/Game/InputActions/IA_Sprint`
  (params (ActionValue :type Boolean) (ElapsedSeconds :type "Float (double-precision)") (TriggeredSeconds :type "Float (double-precision)") (InputAction :type "InputAction Object Reference" :default "/Game/InputActions/IA_Sprint.IA_Sprint"))
  ; Movement
  (:`Started`
    (bind _isa (`/Engine/EditorBlueprintResources/StandardMacros.FlipFlop` :!label _label_2)
      (:`A`
        _)
      (:`B`
        _))
    (`self.Set Is Sprinting` _isa))
  (:`Completed`
    (goto _label_2)))

(event `Key|E`
  (params (Key :type "Key Structure"))
  (bind _interactiontarget (`self.InteractionTarget`))
  ; Interact
  (:`Pressed`
    (`/Engine/EditorBlueprintResources/StandardMacros.IsValid` _interactiontarget
      (:`Is Valid`
        (`self.OnInteract` _interactiontarget)))))

(fn `Get Health Percentage`
  (returns (Value :type "Float (double-precision)"))
  (return (`KismetMathLibrary.SafeDivide` (`self.CurrentHealth`) (`/Game/Lessons/Lesson4/ExtraContent/BP_Lab4CharacterData.MaxHealth` (`self.CharacterData`)))))

(fn `Get Stamina Percentage`
  (returns (Value :type "Float (double-precision)"))
  (return (`KismetMathLibrary.SafeDivide` (`self.CurrentStamina`) (`/Game/Lessons/Lesson4/ExtraContent/BP_Lab4CharacterData.MaxStamina` (`self.CharacterData`)))))

(fn `Set Health`
  (params (Value :type "Float (double-precision)"))
  (returns (NewValue :type "Float (double-precision)"))
  (bind _output_get (set `self.CurrentHealth` (`KismetMathLibrary.FClamp` Value 0.0 (`/Game/Lessons/Lesson4/ExtraContent/BP_Lab4CharacterData.MaxHealth` (`self.CharacterData`)))))
  (`self.OnHealthChange` (`self.Get Health Percentage`))
  (return _output_get))

(fn `Set Interaction Target`
  (params (NewTarget :type "/Game/Lessons/Lesson5/ExtraContent/BP_Lab5Item Object Reference"))
  (if (!= (`self.InteractionTarget`) NewTarget)
    (bind _output_get (set `self.InteractionTarget` NewTarget))
    (`self.OnInteractTargetChange` _output_get)))

(fn `Set Is Sprinting`
  (params (`Is Sprinting` :type Boolean))
  (bind _basespeed (`/Game/Lessons/Lesson4/ExtraContent/BP_Lab4CharacterData.BaseSpeed` (`self.CharacterData`)))
  (bind _output_get (set `self.IsSprinting` `Is Sprinting`))
  (set `CharacterMovementComponent.MaxWalkSpeed` (`KismetMathLibrary.SelectFloat` (* _basespeed 3.0) _basespeed _output_get) (`self.CharacterMovement`)))

(fn `Set Stamina`
  (params (Value :type "Float (double-precision)"))
  (set `self.CurrentStamina` (`KismetMathLibrary.FClamp` Value 0.0 (`/Game/Lessons/Lesson4/ExtraContent/BP_Lab4CharacterData.MaxStamina` (`self.CharacterData`))))
  (`self.OnStaminaChange` (`self.Get Stamina Percentage`)))

(fn `UserConstructionScript`)