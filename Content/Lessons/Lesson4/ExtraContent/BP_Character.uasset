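; Playable lesson character whose mesh, speeds, jump and health/stamina limits come from a swappable CharacterData asset.
; Initialize async-loads the model, then reapplies movement and stats; three debug keys swap data assets and rerun it.
; Enhanced Input drives camera-relative movement, look, jump and sprint, which flips on press and release to triple base speed.
; Health and stamina setters clamp to the data's maximums and report percentage changes.
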(event Custom|Initialize
  (bind _characterdata (Variables|Default|GetCharacterData))
  (bind _model (Variables|/Game/Lessons/Lesson4/ExtraContent/BP_CharacterData.BP_CharacterData_C|GetModel _characterdata))
  ;[0.15 0.15 0.15 0.5] Initialization
  (Utilities|AsyncLoadAsset _model
    (:Completed
      (Components|SkeletalMesh|SetSkeletalMeshAsset (Variables|Character|GetMesh) (Utilities|ResolveSoftReference _model))
      (Variables|/Script/Engine.CharacterMovementComponent|SetJumpZVelocity (Variables|Character|GetCharacterMovement) (Variables|/Game/Lessons/Lesson4/ExtraContent/BP_CharacterData.BP_CharacterData_C|GetJumpSpeed (Variables|Default|GetCharacterData)))
      (Movement|SetIsSprinting (Variables|Movement|GetIsSprinting))
      (Stats|SetHealth (Variables|Stats|GetCurrentHealth))
      (Stats|SetStamina (Variables|Stats|GetCurrentStamina)))))

(event EventBeginPlay
  ;[0.15 0.15 0.15 0.5] Initialization
  (bind _asplayer_controller (Utilities|Casting|CastToPlayerController (Pawn|GetController)))
  (Input|AddMappingContext (PlayerController|LocalPlayerSubsystems|GetEnhancedInputLocalPlayerSubsystem _asplayer_controller) "/Game/Lessons/Lesson2/ExtraContent/InputActions/InputMappingContext.InputMappingContext" 0 "(bIgnoreAllPressedKeysUntilRelease=True,bForceImmediately=False,bNotifyUserSettings=False)")
  (CallFunction|Initialize))

(event Input|EnhancedActionEvents|EnhancedInputActionIA_Sprint
  (params (ActionValue :type Boolean) (ElapsedSeconds :type Float%20%28double-precision%29) (TriggeredSeconds :type Float%20%28double-precision%29) (InputAction :type Input%20Action%20Object%20Reference :default "/Game/Lessons/Lesson2/ExtraContent/InputActions/IA_Sprint.IA_Sprint"))
  ;[0.15 0.15 0.15 0.5] Movement
  (:Started
    (bind _isa (Utilities|FlowControl|FlipFlop :!label _label)
      (:A
        _)
      (:B
        _))
    (Movement|SetIsSprinting _isa))
  (:Completed
    (goto _label)))

(event Input|EnhancedActionEvents|EnhancedInputActionIA_Jump
  (params (ActionValue :type Boolean) (ElapsedSeconds :type Float%20%28double-precision%29) (TriggeredSeconds :type Float%20%28double-precision%29) (InputAction :type Input%20Action%20Object%20Reference :default "/Game/Lessons/Lesson2/ExtraContent/InputActions/IA_Jump.IA_Jump"))
  ;[0.15 0.15 0.15 0.5] Movement
  (:Started
    (Character|Jump))
  (:Completed
    (Character|StopJumping)))

(event Input|EnhancedActionEvents|EnhancedInputActionIA_Move_UD
  (params (ActionValue :type Float%20%28double-precision%29) (ElapsedSeconds :type Float%20%28double-precision%29) (TriggeredSeconds :type Float%20%28double-precision%29) (InputAction :type Input%20Action%20Object%20Reference :default "/Game/Lessons/Lesson2/ExtraContent/InputActions/IA_Move_UD.IA_Move_UD"))
  ;[0.15 0.15 0.15 0.5] Movement
  (:Triggered
    (Pawn|Input|AddMovementInput (Transformation|GetActorForwardVector (Game|GetPlayerCameraManager 0)) ActionValue false)
    (Variables|/Script/Engine.CharacterMovementComponent|SetbOrientRotationToMovement (Variables|Character|GetCharacterMovement) (not (or (!= ActionValue 0.0) (!= (stale Input|EnhancedActionEvents|EnhancedInputActionIA_Move_LR ActionValue) 0.0))) :!label _label))
  (:Completed
    (goto _label)))

(event Input|EnhancedActionEvents|EnhancedInputActionIA_Move_LR
  (params (ActionValue :type Float%20%28double-precision%29) (ElapsedSeconds :type Float%20%28double-precision%29) (TriggeredSeconds :type Float%20%28double-precision%29) (InputAction :type Input%20Action%20Object%20Reference :default "/Game/Lessons/Lesson2/ExtraContent/InputActions/IA_Move_LR.IA_Move_LR"))
  ;[0.15 0.15 0.15 0.5] Movement
  (:Triggered
    (Pawn|Input|AddMovementInput (Transformation|GetActorRightVector (Game|GetPlayerCameraManager 0)) ActionValue false)
    (Variables|/Script/Engine.CharacterMovementComponent|SetbOrientRotationToMovement (Variables|Character|GetCharacterMovement) (not (or (!= (stale Input|EnhancedActionEvents|EnhancedInputActionIA_Move_UD ActionValue) 0.0) (!= ActionValue 0.0))) :!label _label))
  (:Completed
    (goto _label)))

(event Input|EnhancedActionEvents|EnhancedInputActionIA_Look_Yaw
  (params (ActionValue :type Float%20%28double-precision%29) (ElapsedSeconds :type Float%20%28double-precision%29) (TriggeredSeconds :type Float%20%28double-precision%29) (InputAction :type Input%20Action%20Object%20Reference :default "/Game/Lessons/Lesson2/ExtraContent/InputActions/IA_Look_Yaw.IA_Look_Yaw"))
  ;[0.15 0.15 0.15 0.5] Movement
  (Pawn|Input|AddControllerYawInput ActionValue))

(event Input|EnhancedActionEvents|EnhancedInputActionIA_Look_Pitch
  (params (ActionValue :type Float%20%28double-precision%29) (ElapsedSeconds :type Float%20%28double-precision%29) (TriggeredSeconds :type Float%20%28double-precision%29) (InputAction :type Input%20Action%20Object%20Reference :default "/Game/Lessons/Lesson2/ExtraContent/InputActions/IA_Look_Pitch.IA_Look_Pitch"))
  ;[0.15 0.15 0.15 0.5] Movement
  (Pawn|Input|AddControllerPitchInput ActionValue))

(event Input|KeyboardEvents|DebugKey1
  (params (Key :type Key%20Structure :default "None") (ActionValue :type Input%20Action%20Value%20Structure))
  (:Pressed
    (Variables|Default|SetCharacterData "/Game/Data/DA_Character1.DA_Character1")
    (CallFunction|Initialize)))

(event Input|KeyboardEvents|DebugKey2
  (params (Key :type Key%20Structure :default "None") (ActionValue :type Input%20Action%20Value%20Structure))
  (:Pressed
    (Variables|Default|SetCharacterData "/Game/Data/DA_Character2.DA_Character2")
    (CallFunction|Initialize)))

(event Input|KeyboardEvents|DebugKey3
  (params (Key :type Key%20Structure :default "None") (ActionValue :type Input%20Action%20Value%20Structure))
  (:Pressed
    (Variables|Default|SetCharacterData "/Game/Data/DA_Character3.DA_Character3")
    (CallFunction|Initialize)))

(fn ConstructionScript)

(fn SetHealth
  (params (Value :type Float%20%28double-precision%29))
  (bind _output_get (Variables|Stats|SetCurrentHealth (Math|Float|Clamp(Float) Value 0.0 (Variables|/Game/Lessons/Lesson4/ExtraContent/BP_CharacterData.BP_CharacterData_C|GetMaxHealth (Variables|Default|GetCharacterData)))))
  (Default|CallOnHealthChange (Stats|GetHealthPercentage))
  (return _output_get))

(fn SetStamina
  (params (Value :type Float%20%28double-precision%29))
  (Variables|Stats|SetCurrentStamina (Math|Float|Clamp(Float) Value 0.0 (Variables|/Game/Lessons/Lesson4/ExtraContent/BP_CharacterData.BP_CharacterData_C|GetMaxStamina (Variables|Default|GetCharacterData))))
  (Default|CallOnStaminaChange (Stats|GetStaminaPercentage)))

(fn SetIsSprinting
  (params (Is%20Sprinting :type Boolean))
  (bind _characterdata (Variables|Default|GetCharacterData))
  (bind _basespeed (Variables|/Game/Lessons/Lesson4/ExtraContent/BP_CharacterData.BP_CharacterData_C|GetBaseSpeed _characterdata))
  (bind _output_get (Variables|Movement|SetIsSprinting Is%20Sprinting))
  (Variables|/Script/Engine.CharacterMovementComponent|SetMaxWalkSpeed (Variables|Character|GetCharacterMovement) (Math|Float|SelectFloat (* _basespeed 3.0) _basespeed _output_get)))

(fn GetHealthPercentage
  (return (Math|Float|SafeDivide (Variables|Stats|GetCurrentHealth) (Variables|/Game/Lessons/Lesson4/ExtraContent/BP_CharacterData.BP_CharacterData_C|GetMaxHealth (Variables|Default|GetCharacterData)))))

(fn GetStaminaPercentage
  (return (Math|Float|SafeDivide (Variables|Stats|GetCurrentStamina) (Variables|/Game/Lessons/Lesson4/ExtraContent/BP_CharacterData.BP_CharacterData_C|GetMaxStamina (Variables|Default|GetCharacterData)))))